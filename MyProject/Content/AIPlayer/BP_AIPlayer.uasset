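; AI-controlled hero that plays through a level of streamed modules by hopping between path nodes.
; At each node it kills claimed enemies, collects loot to level up, then greedily plans up to four best-scoring nodes, shown as dots.
; Timelines drive all movement; a failed path search retries when a module reports a level update.
; Overlapping an unstreamed module triggers ragdoll death, then respawn at the current node with only its module streamed in.
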(event `self.ReceiveBeginPlay`
  (`|ExecutionSequence`
    (:`then_0`
      (bind _outactors (`GameplayStatics.GetAllActorsOfClass` "/Game/Modules/Base/BP_Module_Base.BP_Module_Base_C"))
      (bind _output_get (set `self.AllModules` _outactors))
      (for _array_element _output_get
        (add `/Game/Modules/Base/BP_Module_Base.LevelUpdated` _array_element (delegate `LevelUpdated_Event`))))
    (:`then_1`
      (`self.K2_SetActorLocation` (`self.K2_GetActorLocation` (`self.CurrentNode`))))
    (:`then_2`
      (bind _asbp_game_mode (cast `/Game/Controller/BP_GameMode` (`GameplayStatics.GetGameMode`)))
      (set `self.GameMode` _asbp_game_mode))
    (:`then_3`
      (`KismetSystemLibrary.Delay` 0.1)
      (`/Game/Controller/BP_GameMode.SetBannerForDuration` (`self.GameMode`) "NewEnumerator1" 2.0)
      (`KismetSystemLibrary.Delay` 2.0)
      (`/Game/Controller/BP_GameMode.SetBannerForDuration` (`self.GameMode`) "NewEnumerator2" 1.5)
      (`KismetSystemLibrary.Delay` 1.5)
      (`/Game/Controller/BP_GameMode.SetBannerForDuration` (`self.GameMode`) "NewEnumerator3" 1.5)
      (`KismetSystemLibrary.Delay` 2.0)
      (`self.ArriveToNode`))
    (:`then_4`
      (bind _returnvalue (`GameplayStatics.GetActorOfClass` "/Game/Controller/BP_Controller.BP_Controller_C"))
      (set `self.BP_PlayerControllerr` _returnvalue))))

(event `LevelUpdated_Event`
  (if (`self.NoPath`)
    (set `self.NoPath` false)
    (`self.CalculateANewPath`)))

(event `ArriveToNode`
  (`/Game/Modules/Base/BP_PathNode.PlayerVisit` (`self.CurrentNode`))
  (`KismetSystemLibrary.Delay` 0.5)
  (`self.ActionAtNode`))

(event `ActionAtNode`
  (bind (_enemytokill _loot_to_loot) (`self.FindEnemyToKillOrLootToLoot`))
  (bind (_startlocation_x _startlocation_y _startlocation_z) (`KismetMathLibrary.BreakVector` (`self.StartLocation`)))
  (bind (_returnvalue_x _returnvalue_y _returnvalue_z) (`KismetMathLibrary.BreakVector` (`self.K2_GetActorLocation` (`self.CurrentEnemy`))))
  (`/Engine/EditorBlueprintResources/StandardMacros.IsValid` _enemytokill
    (:`Is Valid`
      (set `self.CurrentEnemy` _enemytokill)
      (set `self.StartLocation` (`self.K2_GetActorLocation`))
      (set `self.StartRotation` (`self.K2_GetActorRotation`))
      (set `self.TargetRot` (`KismetMathLibrary.MakeRotator` 0.0 0.0 (`KismetMathLibrary.GetYawPitchFromVector` (`KismetMathLibrary.Normal` (- (`self.K2_GetActorLocation` (`self.CurrentEnemy`)) (`self.K2_GetActorLocation`))))))
      (`TimelineComponent.SetPlayRate` (`self.TL_KillEnemy`) 1.4)
      (`/Game/Sounds/SpatialAudioComp.PlaySpatSound` (`self.SpatialAudioComp_JumpToEnemy`))
      (bind (_direction _lerplocaiton _lerpheight _rotation) (`Timeline|TL_KillEnemy` :!via `PlayFromStart` :!label _label)
        (:`Update`
          (`self.K2_SetActorLocation` (`KismetMathLibrary.MakeVector` (`KismetMathLibrary.Lerp` _startlocation_x _returnvalue_x _lerplocaiton) (`KismetMathLibrary.Lerp` _startlocation_y _returnvalue_y _lerplocaiton) (+ (`KismetMathLibrary.Lerp` _startlocation_z _returnvalue_z _lerplocaiton) (* _lerpheight (`self.JumpHeight`)))))
          (`self.K2_SetActorRotation` (`KismetMathLibrary.RLerp` (`self.StartRotation`) (`self.TargetRot`) _rotation true)))
        (:`Finished`
          (if (not (`self.Dead`))
            (`/Game/Enemy/BP_Enemy.KillEnemy` (`self.CurrentEnemy`))
            (`/Game/Sounds/SpatialAudioComp.PlaySpatSound` (`self.SpatialAudioComp_ImpactEnemy`))
            (`KismetSystemLibrary.Delay` 0.2)
            (if (not (`self.Dead`))
              (`self.ActionAtNode`))))))
    (:`Is Not Valid`
      (`/Engine/EditorBlueprintResources/StandardMacros.IsValid` _loot_to_loot
        (:`Is Valid`
          (set `self.CurrentLoot` _loot_to_loot)
          (set `self.StartLocation` (`self.K2_GetActorLocation`))
          (set `self.StartRotation` (`self.K2_GetActorRotation`))
          (set `self.TargetRot` (`KismetMathLibrary.MakeRotator` 0.0 0.0 (`KismetMathLibrary.GetYawPitchFromVector` (`KismetMathLibrary.Normal` (- (`self.K2_GetActorLocation` (`self.CurrentLoot`)) (`self.K2_GetActorLocation`))))))
          (bind (_direction_2 _rot _movement) (`Timeline|TL_GoToLoot` :!via `PlayFromStart` :!label _label_2)
            (:`Update`
              (`self.K2_SetActorLocation` (`KismetMathLibrary.VLerp` (`self.StartLocation`) (`SceneComponent.K2_GetComponentLocation` (`/Game/Loot/BP_Loot.LootLocation` (`self.CurrentLoot`))) _movement))
              (`self.K2_SetActorRotation` (`KismetMathLibrary.RLerp` (`self.StartRotation`) (`self.TargetRot`) _rot true)))
            (:`Finished`
              (if (not (`self.Dead`))
                (`/Game/Loot/BP_Loot.GetLoot` (`self.CurrentLoot`))
                (`self.LevelUp`)
                (`KismetSystemLibrary.Delay` 0.2)
                (if (not (`self.Dead`))
                  (`self.ActionAtNode`))))))
        (:`Is Not Valid`
          (`self.CalculateANewPath`))))))

(event `StopEnemy`
  (goto _label :!via `Stop`))

(event `LevelUp`
  (bind _levelupscene (`self.LevelupScene`))
  (set `self.Level` (+ (`self.Level`) 1.0))
  (`/Game/Controller/BP_GameMode.SetBannerForDuration` (`self.GameMode`) "NewEnumerator4" 1.0)
  (`/Game/Sounds/SpatialAudioComp.PlaySpatSound` (`self.SpatialAudioComp_LevelUp`))
  (bind (_direction _rotation _scale) (`Timeline|TL_Levelup` :!via `PlayFromStart`)
    (:`Update`
      (`SceneComponent.SetRelativeScale3D` _levelupscene (`KismetMathLibrary.MakeVector` 1.0 1.0 _scale))
      (`SceneComponent.K2_SetRelativeRotation` _levelupscene (`KismetMathLibrary.MakeRotator` 0.0 0.0 _rotation) false false))))

(event `StopLoot`
  (goto _label_2 :!via `Stop`))

(event `CalculateANewPath`
  (bind _foundapath (`self.CalculatePath`))
  (if _foundapath
    (`self.DrawPath`)
    (if (> (`KismetMathLibrary.Vector_Distance` (`self.K2_GetActorLocation`) (`self.K2_GetActorLocation` (`self.CurrentNode`))) 100.0)
      (if (== (`/Game/Modules/Base/BP_PathNode.ConnectedModule` (`self.CurrentNode`)) (`/Game/Modules/Base/BP_PathNode.ConnectedModule` (`|GetArrayItem` (`self.PathNodes`))))
        (`self.WalkToNewNode`)
        (else
          (set `self.StartLocation` (`self.K2_GetActorLocation`))
          (set `self.StartRotation` (`self.K2_GetActorRotation`))
          (set `self.TargetRot` (`KismetMathLibrary.MakeRotator` 0.0 0.0 (`KismetMathLibrary.GetYawPitchFromVector` (`KismetMathLibrary.Normal` (- (`self.K2_GetActorLocation` (`self.CurrentNode`)) (`self.K2_GetActorLocation`))))))
          (bind (_direction _rot _movement) (`Timeline|Timeline` :!via `PlayFromStart` :!label _label_3)
            (:`Update`
              (`self.K2_SetActorLocation` (`KismetMathLibrary.VLerp` (`self.StartLocation`) (`self.K2_GetActorLocation` (`self.CurrentNode`)) _movement))
              (`self.K2_SetActorRotation` (`KismetMathLibrary.RLerp` (`self.StartRotation`) (`self.TargetRot`) _rot true)))
            (:`Finished`
              (if (not (`self.Dead`))
                (`KismetSystemLibrary.Delay` 0.2)
                (if (not (`self.Dead`))
                  (`self.ActionAtNode`)))))))
      (else
        (`self.WalkToNewNode`)))
    (else
      (set `self.NoPath` true))))

(event `StopGoBackToPosition`
  (goto _label_3 :!via `Stop`))

(event `WalkToNewNode`
  (set `self.StartRotation` (`self.K2_GetActorRotation`))
  (set `self.TargetRot` (`KismetMathLibrary.MakeRotator` 0.0 0.0 (`KismetMathLibrary.GetYawPitchFromVector` (`KismetMathLibrary.Normal` (- (`self.K2_GetActorLocation` (`|GetArrayItem` (`self.PathNodes`))) (`self.K2_GetActorLocation`))))))
  (set `self.StartLocation` (`self.K2_GetActorLocation`))
  (`/Game/Sounds/SpatialAudioComp.PlaySpatSound` (`self.SpatialAudioComp_Movement`))
  (bind (_direction _lerp _rot) (`Timeline|TL_Move` :!via `PlayFromStart` :!label _label_4)
    (:`Update`
      (`self.K2_SetActorLocation` (`KismetMathLibrary.VLerp` (`self.StartLocation`) (`self.K2_GetActorLocation` (`|GetArrayItem` (`self.PathNodes`))) _lerp))
      (`self.K2_SetActorRotation` (`KismetMathLibrary.RLerp` (`self.StartRotation`) (`self.TargetRot`) _rot true)))
    (:`Finished`
      (if (not (`self.Dead`))
        (set `self.CurrentNode` (`|GetArrayItem` (`self.PathNodes`)))
        (`self.ArriveToNode`)))))

(event `DrawPath`
  (bind _pathnodes (`self.PathNodes`))
  (bind _distancbetweenpathdots (`self.DistancBetweenPathDots`))
  (bind _startdrawlocation (`self.StartDrawLocation`))
  (bind _all_path_renders (`self.All Path renders`))
  (`self.K2_DestroyActor` _all_path_renders)
  (`KismetArrayLibrary.Array_Clear` _all_path_renders)
  (set `self.StartDrawLocation` (`self.K2_GetActorLocation`))
  (for _array_element (`self.PathNodes`)
    (bind _returnvalue (`self.K2_GetActorLocation` _array_element))
    (bind _returnvalue_2 (`KismetMathLibrary.Vector_Distance` _startdrawlocation _returnvalue))
    (for _index (range (+ (`KismetMathLibrary.FTrunc` (/ _returnvalue_2 _distancbetweenpathdots)) 1))
      (bind _returnvalue_3 (`|SpawnActorFromClass` "/Game/AIPlayer/BP_Path.BP_Path_C" (`KismetMathLibrary.MakeTransform` (`KismetMathLibrary.VLerp` _startdrawlocation _returnvalue (/ (* _index _distancbetweenpathdots) _returnvalue_2))) "Undefined" "MultiplyWithRoot" null null))
      (`KismetArrayLibrary.Array_Add` (`self.All Path renders`) _returnvalue_3))
    (set `self.StartDrawLocation` _returnvalue))
  (bind _returnvalue_4 (`|SpawnActorFromClass` "/Game/AIPlayer/BP_Path.BP_Path_C" (`KismetMathLibrary.MakeTransform` (`self.K2_GetActorLocation` (`|GetArrayItem` _pathnodes (`KismetArrayLibrary.Array_LastIndex` _pathnodes)))) "Undefined" "MultiplyWithRoot" null null))
  (`KismetArrayLibrary.Array_Add` (`self.All Path renders`) _returnvalue_4)
  (`/Game/AIPlayer/BP_Path.IsLastPosition` _returnvalue_4))

(event `StopMoveTL`
  (goto _label_4 :!via `Stop`))

(event `self.Sphere.OnComponentBeginOverlap`
  (params (OverlappedComponent :type "PrimitiveComponent Object Reference") (OtherActor :type "Actor Object Reference") (OtherComp :type "PrimitiveComponent Object Reference") (OtherBodyIndex :type Integer) (bFromSweep :type Boolean) (SweepResult :type "HitResult Structure (by ref)"))
  (bind _all_path_renders (`self.All Path renders`))
  (bind _hero_heroson (`self.hero_heroson`))
  (bind _asbp_module_base (cast `/Game/Modules/Base/BP_Module_Base` OtherActor))
  (if (not (`/Game/Modules/Base/BP_Module_Base.IsStreamedIn` _asbp_module_base))
    (`/Game/Sounds/SpatialAudioComp.PlaySpatSound` (`self.SpatialAudioComp_FallIntoVoid`))
    (`PlayerController.SetViewTargetWithBlend` (`GameplayStatics.GetPlayerController` 0) (`self.DeathCamera`) 1.0 "VTBlend_Cubic" 0.0 false)
    (set `self.Dead` true)
    (`PrimitiveComponent.SetSimulatePhysics` _hero_heroson true)
    (`PrimitiveComponent.SetCollisionEnabled` _hero_heroson "QueryAndPhysics")
    (`self.StopGoBackToPosition`)
    (`self.StopMoveTL`)
    (`self.StopLoot`)
    (`self.StopEnemy`)
    (`self.K2_DestroyActor` _all_path_renders)
    (`KismetArrayLibrary.Array_Clear` _all_path_renders)
    (`KismetSystemLibrary.Delay` 3.0)
    (`self.Respawn`)))

(event `Respawn`
  (bind _currentnode (`self.CurrentNode`))
  (bind _hero_heroson (`self.hero_heroson`))
  (`/Game/Sounds/SpatialAudioComp.PlaySpatSound` (`self.SpatialAudioComp_Respawn`))
  (`/Game/Modules/Base/BP_Module_Base.StreamOutLevel` (`self.AllModules`))
  (`/Game/Modules/Base/BP_Module_Base.StreamInLevel` (`/Game/Modules/Base/BP_PathNode.ConnectedModule` _currentnode))
  (`KismetSystemLibrary.Delay` 1.0)
  (`PrimitiveComponent.SetSimulatePhysics` _hero_heroson false)
  (`SceneComponent.K2_AttachToComponent` _hero_heroson (`self.DefaultSceneRoot`) "None" "SnapToTarget" "SnapToTarget" "KeepRelative" true)
  (`SceneComponent.K2_SetRelativeRotation` (`self.hero_heroson`) (struct :`Yaw` -90.0) false false)
  (`SceneComponent.K2_SetRelativeRotation` (`self.hero_heroson`) (struct :`Yaw` -90.0) false false)
  (`self.K2_SetActorLocation` (`self.K2_GetActorLocation` _currentnode))
  (`PlayerController.SetViewTargetWithBlend` (`GameplayStatics.GetPlayerController` 0) (`self.BP_PlayerControllerr`) 1.0 "VTBlend_Cubic" 0.0 false)
  (`KismetSystemLibrary.Delay` 2.0)
  (set `self.Dead` false)
  (`self.ArriveToNode`))

(fn `CalculateBestPoint`
  (params (NodeToEvaluate :type "/Game/Modules/Base/BP_PathNode Object Reference"))
  (returns (BestPathNode :type "/Game/Modules/Base/BP_PathNode Object Reference"))
  (locals (HighestPoints :type "Float (double-precision)") (BestNextNode :type "/Game/Modules/Base/BP_PathNode Object Reference"))
  (set `local.HighestPoints` -220.0)
  (set `local.BestNextNode` null)
  (for _array_element (`/Game/Modules/Base/BP_PathNode.ConnectedPathNodes` NodeToEvaluate)
    (bind (_points _isvalid) (`/Game/Modules/Base/BP_PathNode.Evaluate` _array_element))
    (if (and (> _points (`local.HighestPoints`)) _isvalid (not (`KismetArrayLibrary.Array_Contains` (`self.PathNodes`) _array_element)) (!= _array_element (`self.CurrentNode`)))
      (set `local.HighestPoints` _points)
      (set `local.BestNextNode` _array_element)))
  (return (`local.BestNextNode`)))

(fn `CalculatePath`
  (returns (FoundAPath :type Boolean))
  (locals (NewToAdd :type "/Game/Modules/Base/BP_PathNode Object Reference"))
  (bind _newtoadd (`local.NewToAdd`))
  (bind _newtoadd_2 (`local.NewToAdd`))
  (bind _newtoadd_3 (`local.NewToAdd`))
  (bind _newtoadd_4 (`local.NewToAdd`))
  (`KismetArrayLibrary.Array_Clear` (`self.PathNodes`))
  (bind _output_get (set `local.NewToAdd` (`self.CalculateBestPoint` (`self.CurrentNode`))))
  (`/Engine/EditorBlueprintResources/StandardMacros.IsValid` _output_get
    (:`Is Valid`
      (`KismetArrayLibrary.Array_Add` (`self.PathNodes`) _newtoadd_4)
      (`/Game/Modules/Base/BP_PathNode.Claim` _newtoadd_4)
      (bind _output_get_2 (set `local.NewToAdd` (`self.CalculateBestPoint` (`local.NewToAdd`))))
      (`/Engine/EditorBlueprintResources/StandardMacros.IsValid` _output_get_2
        (:`Is Valid`
          (`KismetArrayLibrary.Array_Add` (`self.PathNodes`) _newtoadd)
          (`/Game/Modules/Base/BP_PathNode.Claim` _newtoadd)
          (bind _output_get_3 (set `local.NewToAdd` (`self.CalculateBestPoint` (`local.NewToAdd`))))
          (`/Engine/EditorBlueprintResources/StandardMacros.IsValid` _output_get_3
            (:`Is Valid`
              (`KismetArrayLibrary.Array_Add` (`self.PathNodes`) _newtoadd_2)
              (`/Game/Modules/Base/BP_PathNode.Claim` _newtoadd_2)
              (bind _output_get_4 (set `local.NewToAdd` (`self.CalculateBestPoint` (`local.NewToAdd`))))
              (`/Engine/EditorBlueprintResources/StandardMacros.IsValid` _output_get_4
                (:`Is Valid`
                  (`KismetArrayLibrary.Array_Add` (`self.PathNodes`) _newtoadd_3)
                  (`/Game/Modules/Base/BP_PathNode.Claim` _newtoadd_3))
                (:`Is Not Valid`
                  _)))
            (:`Is Not Valid`
              _)))
        (:`Is Not Valid`
          _))
      (return true))
    (:`Is Not Valid`
      (return false))))

(fn `FindEnemyToKillOrLootToLoot`
  (returns (EnemyToKill :type "/Game/Enemy/BP_Enemy Object Reference") (`Loot to loot` :type "/Game/Loot/BP_Loot Object Reference"))
  (bind _currentnode (`self.CurrentNode`))
  (for _array_element (`/Game/Modules/Base/BP_PathNode.ClaimedEnemies` _currentnode)
    (if (not (`/Game/Enemy/BP_Enemy.Dead` _array_element))
      (return _array_element null)))
  (for _array_element_2 (`/Game/Modules/Base/BP_PathNode.ClaimedLoot` _currentnode)
    (if (and (not (`/Game/Loot/BP_Loot.HasBeenLooted` _array_element_2)) (`/Game/Loot/BP_Loot.IsLootable` _array_element_2))
      (return null _array_element_2)))
  (return null null))

(fn `UserConstructionScript`)