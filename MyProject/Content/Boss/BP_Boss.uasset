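; Mushroom boss that hunts the AI player across path nodes and attacks on reaching it.
; After a spawn delay it drops in during a camera cutscene, its camera smoothly tracking the mesh.
; It greedily hops to the unscanned connected node nearest the player, clearing the scanned list at dead ends.
; Upon meeting, a timeline-driven leap triggers Niagara effects and kills the player if the boss's level is higher.
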(event `Spawn`
  (`PlayerController.SetViewTargetWithBlend` (`GameplayStatics.GetPlayerController` 0) self 1.0 "VTBlend_Cubic" 0.0 false)
  (`SceneComponent.SetHiddenInGame` (`self.shroom_boss`) false false)
  (bind (_direction _droplerp) (`Timeline|TL_Spawnm` :!via `PlayFromStart`)
    (:`Update`
      (`SceneComponent.K2_SetRelativeLocation` (`self.shroom_boss`) (`KismetMathLibrary.MakeVector` 0.0 0.0 (* (- 1.0 _droplerp) 1000.0)) false false))
    (:`Finished`
      (`KismetSystemLibrary.Delay` 1.5)
      (`PlayerController.SetViewTargetWithBlend` (`GameplayStatics.GetPlayerController` 0) (`self.BPController`) 1.0 "VTBlend_Cubic" 0.0 false)
      (`KismetSystemLibrary.Delay` 1.5)
      (`self.CalculatePath`))))

(event `self.ReceiveBeginPlay`
  (`|ExecutionSequence`
    (:`then_0`
      (bind _outactors (`GameplayStatics.GetAllActorsOfClass` "/Game/Modules/Base/BP_PathNode.BP_PathNode_C"))
      (set `self.PathNodes` _outactors))
    (:`then_1`
      (bind _returnvalue (`GameplayStatics.GetActorOfClass` "/Game/AIPlayer/BP_AIPlayer.BP_AIPlayer_C"))
      (set `self.AIPlayer` _returnvalue))
    (:`then_2`
      (bind _returnvalue_2 (`GameplayStatics.GetActorOfClass` "/Game/Controller/BP_Controller.BP_Controller_C"))
      (set `self.BPController` _returnvalue_2))
    (:`then_3`
      (`self.K2_SetActorLocation` (`self.K2_GetActorLocation` (`self.CurrentNode`))))
    (:`then_4`
      (`KismetSystemLibrary.Delay` (`self.SpawnDelay`))
      (`self.Spawn`))))

(event `self.ReceiveTick`
  (params (DeltaSeconds :type "Float (single-precision)"))
  (bind _camera (`self.Camera`))
  (bind _camera_2 (`self.Camera`))
  (bind (_yaw _pitch) (`KismetMathLibrary.GetYawPitchFromVector` (`KismetMathLibrary.Normal` (- (`SceneComponent.K2_GetComponentLocation` (`self.shroom_boss`)) (`SceneComponent.K2_GetComponentLocation` (`self.Camera`))))))
  (`SceneComponent.K2_SetWorldLocation` _camera (`KismetMathLibrary.VInterpTo` (`SceneComponent.K2_GetComponentLocation` _camera) (`SceneComponent.K2_GetComponentLocation` (`self.Scene`)) DeltaSeconds 1.0) false false)
  (`SceneComponent.K2_SetWorldRotation` _camera_2 (`KismetMathLibrary.RInterpTo` (`SceneComponent.K2_GetComponentRotation` _camera_2) (`KismetMathLibrary.MakeRotator` 0.0 _pitch _yaw) DeltaSeconds 1.0) false false))

(event `CalculatePath`
  (`KismetArrayLibrary.Array_Add` (`self.ScannedRooms`) (`self.CurrentNode`))
  (set `self.TargetNode` (`self.CalculatePathToPlayer`))
  (`self.Move`))

(event `Move`
  (set `self.StartLocation` (`self.K2_GetActorLocation`))
  (set `self.StartRotation` (`self.K2_GetActorRotation`))
  (set `self.TargetRot` (`KismetMathLibrary.MakeRotator` 0.0 0.0 (`KismetMathLibrary.GetYawPitchFromVector` (`KismetMathLibrary.Normal` (- (`self.K2_GetActorLocation` (`self.TargetNode`)) (`self.K2_GetActorLocation`))))))
  (bind (_direction _movelerp) (`Timeline|TL_Move` :!via `PlayFromStart`)
    (:`Update`
      (`self.K2_SetActorLocation` (`KismetMathLibrary.VLerp` (`self.StartLocation`) (`self.K2_GetActorLocation` (`self.TargetNode`)) _movelerp))
      (`self.K2_SetActorRotation` (`KismetMathLibrary.RLerp` (`self.StartRotation`) (`self.TargetRot`) 0.0 true)))
    (:`Finished`
      (set `self.CurrentNode` (`self.TargetNode`))
      (if (or (== (`/Game/Modules/Base/BP_PathNode.ConnectedModule` (`self.CurrentNode`)) (`/Game/Modules/Base/BP_PathNode.ConnectedModule` (`/Game/AIPlayer/BP_AIPlayer.CurrentNode` (`self.AIPlayer`)))) (== (`/Game/Modules/Base/BP_PathNode.ConnectedModule` (`self.CurrentNode`)) (`|GetArrayItem` (`/Game/AIPlayer/BP_AIPlayer.PathNodes` (`self.AIPlayer`)))))
        (`self.EpicFight`)
        (else
          (`KismetSystemLibrary.Delay` 2.0)
          (`self.CalculatePath`))))))

(event `EpicFight`
  (bind (_startlocation_x _startlocation_y _startlocation_z) (`KismetMathLibrary.BreakVector` (`self.StartLocation`)))
  (bind (_returnvalue_x _returnvalue_y _returnvalue_z) (`KismetMathLibrary.BreakVector` (`self.K2_GetActorLocation` (`self.AIPlayer`))))
  (`/Game/AIPlayer/BP_AIPlayer.Getting Attacked` (`self.AIPlayer`))
  (set `self.StartLocation` (`self.K2_GetActorLocation`))
  (set `self.StartRotation` (`self.K2_GetActorRotation`))
  (set `self.TargetRot` (`KismetMathLibrary.MakeRotator` 0.0 0.0 (`KismetMathLibrary.GetYawPitchFromVector` (`KismetMathLibrary.Normal` (- (`self.K2_GetActorLocation` (`self.AIPlayer`)) (`self.K2_GetActorLocation`))))))
  (bind (_direction _lerplocaiton _lerpheight _rotation) (`Timeline|Timeline` :!via `PlayFromStart`)
    (:`Update`
      (`self.K2_SetActorLocation` (`KismetMathLibrary.MakeVector` (`KismetMathLibrary.Lerp` _startlocation_x _returnvalue_x _lerplocaiton) (`KismetMathLibrary.Lerp` _startlocation_y _returnvalue_y _lerplocaiton) (+ (`KismetMathLibrary.Lerp` _startlocation_z _returnvalue_z _lerplocaiton) (* _lerpheight (`self.JumpHeight`)))))
      (`self.K2_SetActorRotation` (`KismetMathLibrary.RLerp` (`self.StartRotation`) (`self.TargetRot`) _rotation true)))
    (:`Finished`
      (`ActorComponent.Activate` (`self.NS_BossFight`) true)
      (`KismetSystemLibrary.Delay` 0.5)
      (`ActorComponent.Activate` (`self.NS_BossFight1`) true)
      (`KismetSystemLibrary.Delay` 0.2)
      (if (> (`self.BossLevel`) (`/Game/AIPlayer/BP_AIPlayer.Level` (`self.AIPlayer`)))
        (`/Game/AIPlayer/BP_AIPlayer.KillPlayer` (`self.AIPlayer`) false)))))

(fn `CalculatePathToPlayer`
  (returns (TargetNode :type "/Game/Modules/Base/BP_PathNode Object Reference"))
  (locals (DiscardedLocations :type "Array of /Game/Modules/Base/BP_PathNode Object Reference") (ClosestToPlayer :type "/Game/Modules/Base/BP_PathNode Object Reference") (DistanceToPlayer :type "Float (double-precision)"))
  (bind _closesttoplayer (`local.ClosestToPlayer`))
  (set `local.DistanceToPlayer` 999999.0)
  (for _array_element (`/Game/Modules/Base/BP_PathNode.ConnectedPathNodes` (`self.CurrentNode`)) :!label _label
    (bind _returnvalue (`self.GetDistanceTo` _array_element (`self.AIPlayer`)))
    (if (and (< _returnvalue (`local.DistanceToPlayer`)) (not (`KismetArrayLibrary.Array_Contains` (`self.ScannedRooms`) _array_element)))
      (set `local.DistanceToPlayer` _returnvalue)
      (set `local.ClosestToPlayer` _array_element)))
  (`/Engine/EditorBlueprintResources/StandardMacros.IsValid` _closesttoplayer
    (:`Is Valid`
      (return _closesttoplayer))
    (:`Is Not Valid`
      (`KismetArrayLibrary.Array_Clear` (`self.ScannedRooms`))
      (goto _label))))

(fn `UserConstructionScript`)