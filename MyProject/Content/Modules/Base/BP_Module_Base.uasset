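; Base module actor that fakes streaming in and out by swapping two scenes through scale and visibility, toggled on Click.
; BeginPlay gathers child SubStreamer components, then after a short delay snaps everything to the LevelLoaded state.
; One timeline, played forward or reversed, scales both scenes, flips visibility and triggers SubStreamers with index-staggered delays.
; It also collects unique loot and enemy references, though HasLoot and HasEnemy are empty stubs.
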(event `self.ReceiveBeginPlay`
  (bind _levelloaded (`self.LevelLoaded`))
  (bind _levelloaded_2 (`self.LevelLoaded`))
  (bind _substreamers (`self.SubStreamers`))
  (`|ExecutionSequence`
    (:`then_0`
      (for _array_element (`SceneComponent.GetChildrenComponents` (`self.DefaultSceneRoot`) true)
        (bind _assub_streamer (cast `/Game/Modules/Base/SubStreamer` _array_element))
        (`KismetArrayLibrary.Array_AddUnique` (`self.SubStreamers`) _assub_streamer)))
    (:`then_1`
      (set `self.InitialStreamedInSceneScale` (`SceneComponent.RelativeScale3D` (`self.StreamedInScene`)))
      (set `self.InitialStreamedOutSceneScale` (`SceneComponent.RelativeScale3D` (`self.StreamedOutScene`))))
    (:`then_2`
      (`KismetSystemLibrary.Delay` 0.1)
      (`|ExecutionSequence`
        (:`then_0`
          (`SceneComponent.SetRelativeScale3D` (`self.StreamedInScene`) (* (`KismetMathLibrary.Conv_BoolToDouble` _levelloaded) (`self.InitialStreamedInSceneScale`)))
          (`SceneComponent.SetRelativeScale3D` (`self.StreamedOutScene`) (* (`KismetMathLibrary.Conv_BoolToDouble` (not _levelloaded)) (`self.InitialStreamedOutSceneScale`))))
        (:`then_1`
          (`SceneComponent.SetHiddenInGame` (`self.StreamedOutScene`) _levelloaded_2 true)
          (`SceneComponent.SetHiddenInGame` (`self.StreamedInScene`) (not _levelloaded_2) true))
        (:`then_2`
          (if (`self.LevelLoaded`)
            (`/Game/Modules/Base/SubStreamer.StreamIn` _substreamers 0.0 true)
            (else
              (`/Game/Modules/Base/SubStreamer.StreamOut` _substreamers 0.0 true)
              (`TimelineComponent.SetNewTime` (`self.TL_ShrinkLevel`) 1.7))))))))

(event `StreamOutLevel`
  (bind _substreamers (`self.SubStreamers`))
  (bind _substreamers_2 (`self.SubStreamers`))
  (set `self.LevelLoaded` false)
  (bind (_direction _streaminscenescale _streamoutscenescale) (`Timeline|TL_ShrinkLevel` :!label _label)
    (:`Update`
      (`SceneComponent.SetRelativeScale3D` (`self.StreamedInScene`) (* _streaminscenescale (`self.InitialStreamedInSceneScale`)))
      (`SceneComponent.SetRelativeScale3D` (`self.StreamedOutScene`) (* _streamoutscenescale (`self.InitialStreamedOutSceneScale`))))
    (:`TriggerSubStreamOut`
      (switch `ETimelineDirection` _direction
        (:`Forward`
          (for (_array_element _array_index) _substreamers_2
            (`/Game/Modules/Base/SubStreamer.StreamOut` _array_element (`KismetMathLibrary.MapRangeClamped` (`KismetMathLibrary.Conv_IntToDouble` _array_index) 0.0 (`KismetMathLibrary.Conv_IntToDouble` (`KismetArrayLibrary.Array_Length` _substreamers_2)) 0.0 0.3) false)))))
    (:`TriggerSubStreamIn`
      (switch `ETimelineDirection` _direction
        (:`Backward`
          (for (_array_element_2 _array_index_2) _substreamers
            (`/Game/Modules/Base/SubStreamer.StreamIn` _array_element_2 (`KismetMathLibrary.MapRangeClamped` (`KismetMathLibrary.Conv_IntToDouble` _array_index_2) 0.0 (`KismetMathLibrary.Conv_IntToDouble` (`KismetArrayLibrary.Array_Length` _substreamers)) 0.0 0.3) false)))))
    (:`ToggleHidden`
      (switch `ETimelineDirection` _direction
        (:`Forward`
          (`SceneComponent.SetHiddenInGame` (`self.StreamedOutScene`) false true)
          (`SceneComponent.SetHiddenInGame` (`self.StreamedInScene`) true true))
        (:`Backward`
          (`SceneComponent.SetHiddenInGame` (`self.StreamedOutScene`) true true)
          (`SceneComponent.SetHiddenInGame` (`self.StreamedInScene`) false true))))))

(event `StreamInLevel`
  (set `self.LevelLoaded` true)
  (goto _label :!via `Reverse`))

(event `AddLoot`
  (params (Loot :type "/Game/Loot/BP_Loot Object Reference"))
  (`KismetArrayLibrary.Array_AddUnique` (`self.Loot`) Loot))

(event `AddEnemy`
  (params (Enemy :type "/Game/Enemy/BP_Enemy Object Reference"))
  (`KismetArrayLibrary.Array_AddUnique` (`self.Enemies`) Enemy))

(event `/Game/Controller/ClickInterface.Click`
  (if (`self.LevelLoaded`)
    (`self.StreamOutLevel`)
    (else
      (`self.StreamInLevel`))))

(fn `HasEnemy`
  (return))

(fn `HasLoot`)

(fn `IsStreamedIn`
  (returns (LevelLoaded :type Boolean))
  (return (`self.LevelLoaded`)))

(fn `UserConstructionScript`)