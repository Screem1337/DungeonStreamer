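; BP_PathNode is a path node tied to a module that scores itself as a destination to visit, valid only while that module is streamed in.
; The score rewards available living enemies and lootable items, penalizes repeat and recent visits, and adds a bonus for a lone unvisited node.
; Available targets exclude those claimed by connected nodes, and Claim stores the remainder as this node's own.
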(event `self.ReceiveBeginPlay`
  (bind _outactors (`GameplayStatics.GetAllActorsOfClass` "BP_PathNode_C"))
  (set `self.AllPathNodes` _outactors))

(event `PlayerVisit`
  (`/Engine/EditorBlueprintResources/StandardMacros.IncrementInt` (`self.VisitedCount`)
    (:`  `
      (set `self.LastTimeVisited` (`KismetSystemLibrary.GetGameTimeInSeconds`)))))

(fn `AvailableLootAndEnemies`
  (returns (Enemy :type "Array of /Game/Enemy/BP_Enemy Object Reference") (Loot :type "Array of /Game/Loot/BP_Loot Object Reference"))
  (locals (LootThatNodeWantsToClaim :type "Array of /Game/Loot/BP_Loot Object Reference") (EnemiesThatNodeWantsToClaim :type "Array of /Game/Enemy/BP_Enemy Object Reference"))
  (`KismetArrayLibrary.Array_Clear` (`local.LootThatNodeWantsToClaim`))
  (`KismetArrayLibrary.Array_Clear` (`local.EnemiesThatNodeWantsToClaim`))
  (`|ExecutionSequence`
    (:`then_0`
      (for _array_element (`/Game/Modules/Base/BP_Module_Base.Enemies` (`self.ConnectedModule`))
        (if (not (`/Game/Enemy/BP_Enemy.Dead` _array_element))
          (`KismetArrayLibrary.Array_AddUnique` (`local.EnemiesThatNodeWantsToClaim`) _array_element))))
    (:`then_1`
      (for _array_element_2 (`/Game/Modules/Base/BP_Module_Base.Loot` (`self.ConnectedModule`))
        (if (and (not (`/Game/Loot/BP_Loot.HasBeenLooted` _array_element_2)) (`/Game/Loot/BP_Loot.IsLootable` _array_element_2))
          (`KismetArrayLibrary.Array_AddUnique` (`local.LootThatNodeWantsToClaim`) _array_element_2))))
    (:`then_2`
      (for _array_element_3 (`self.ConnectedPathNodes`)
        (for _array_element_4 (`/Game/Modules/Base/BP_PathNode.ClaimedEnemies` _array_element_3)
          (`KismetArrayLibrary.Array_RemoveItem` (`local.EnemiesThatNodeWantsToClaim`) _array_element_4))
        (for _array_element_5 (`/Game/Modules/Base/BP_PathNode.ClaimedLoot` _array_element_3)
          (`KismetArrayLibrary.Array_RemoveItem` (`local.LootThatNodeWantsToClaim`) _array_element_5))))
    (:`then_3`
      (return (`local.EnemiesThatNodeWantsToClaim`) (`local.LootThatNodeWantsToClaim`)))))

(fn `Claim`
  (bind (_enemy _loot) (`self.AvailableLootAndEnemies`))
  (set `self.ClaimedEnemies` _enemy)
  (set `self.ClaimedLoot` _loot))

(fn `Evaluate`
  (returns (Points :type "Float (double-precision)") (IsValid :type Boolean))
  (locals (Loot :type "Array of /Game/Loot/BP_Loot Object Reference") (Enemy :type "Array of /Game/Enemy/BP_Enemy Object Reference"))
  (bind (_enemy _loot) (`self.AvailableLootAndEnemies`))
  (return (+ (* (`KismetMathLibrary.Conv_IntToDouble` (`KismetArrayLibrary.Array_Length` _enemy)) 0.5) (* (`KismetMathLibrary.Conv_IntToDouble` (`KismetArrayLibrary.Array_Length` _loot)) 1.5) (`KismetMathLibrary.Conv_IntToDouble` (* (`self.VisitedCount`) -1)) (`KismetMathLibrary.MapRangeClamped` (- (`KismetSystemLibrary.GetGameTimeInSeconds`) (`self.LastTimeVisited`)) 1.0 15.0 -5.0) (`KismetMathLibrary.SelectFloat` 5.0 0.0 (and (== (`self.VisitedCount`) 0) (== (`KismetArrayLibrary.Array_Length` (`self.AllPathNodes`)) 1)))) (`/Game/Modules/Base/BP_Module_Base.IsStreamedIn` (`self.ConnectedModule`))))

(fn `UserConstructionScript`)