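; Base actor for level modules that animates its streaming in and out and tracks the LevelLoaded state.
; It gathers child SubStreamer components on BeginPlay and calls each with a value staggered by array index.
; Stream-out triggers the sub-streamers, then after a delay shrinks the actor via timeline and hides it.
; Stream-in unhides it and reverses the timeline, then triggers the sub-streamers after a delay.
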(event `self.ReceiveBeginPlay`
  (`|ExecutionSequence`
    (:`then_0`
      (for _array_element (`SceneComponent.GetChildrenComponents` (`self.DefaultSceneRoot`) false)
        (bind _assub_streamer (cast `/Game/Modules/SubStreamer` _array_element))
        (`KismetArrayLibrary.Array_AddUnique` (`self.SubStreamers`) _assub_streamer)))
    (:`then_1`
      (set `self.InitialScale` (`self.GetActorScale3D`)))))

(event `StreamOutLevel`
  (bind _substreamers (`self.SubStreamers`))
  (for (_array_element _array_index) _substreamers
    (`/Game/Modules/SubStreamer.StreamOut` _array_element (`KismetMathLibrary.MapRangeClamped` (`KismetMathLibrary.Conv_IntToDouble` _array_index) 0.0 (`KismetMathLibrary.Conv_IntToDouble` (`KismetArrayLibrary.Array_Length` _substreamers)) 0.0 0.3)))
  (`KismetSystemLibrary.RetriggerableDelay` 0.5)
  (bind (_direction _scale) (`Timeline|TL_ShrinkLevel` :!label _label)
    (:`Update`
      (`self.SetActorScale3D` (* _scale (`self.InitialScale`))))
    (:`Finished`
      (switch `ETimelineDirection` _direction
        (:`Forward`
          (`self.SetActorHiddenInGame` true)
          (set `self.LevelLoaded` false))))))

(event `StreamInLevel`
  (bind _substreamers (`self.SubStreamers`))
  (`|ExecutionSequence`
    (:`then_0`
      (`self.SetActorHiddenInGame` false)
      (goto _label :!via `Reverse`))
    (:`then_1`
      (`KismetSystemLibrary.RetriggerableDelay` 0.5)
      (for (_array_element _array_index) _substreamers
        (`/Game/Modules/SubStreamer.StreamIn` _array_element (`KismetMathLibrary.MapRangeClamped` (`KismetMathLibrary.Conv_IntToDouble` _array_index) 0.0 (`KismetMathLibrary.Conv_IntToDouble` (`KismetArrayLibrary.Array_Length` _substreamers)) 0.0 0.3)))
      (`KismetSystemLibrary.Delay` 0.5)
      (set `self.LevelLoaded` true))))

(fn `UserConstructionScript`)