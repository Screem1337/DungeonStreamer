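; Loot chest Blueprint whose lid swings open or shut according to its IsLootable flag.
; The Click event toggles IsLootable, so a lootable chest shows as open.
; Tick calls the parent, then eases the lid pivot toward the open or closed rotation with RInterpTo.
; The construction script snaps the lid to the matching pose.
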(event `/Game/Controller/ClickInterface.Click`
  (bind _output_get (set `self.IsLootable` (not (`self.IsLootable`))))
  (set `self.IsLootable` _output_get))

(event `self.ReceiveTick`
  (params (DeltaSeconds :type "Float (single-precision)"))
  (`parent.ReceiveTick` DeltaSeconds)
  (`SceneComponent.K2_SetRelativeRotation` (`self.LidPivot`) (`KismetMathLibrary.RInterpTo` (`SceneComponent.RelativeRotation` (`self.LidPivot`)) (select `bool` (`self.IsLootable`) :`true` (struct :`Roll` -70.0) :!type "Rotator Structure") (`GameplayStatics.GetWorldDeltaSeconds`) 5.0) false false))

(fn `UserConstructionScript`
  (`parent.UserConstructionScript`)
  (`SceneComponent.K2_SetRelativeRotation` (`self.LidPivot`) (select `bool` (`self.IsLootable`) :`true` (struct :`Roll` -70.0) :!type "Rotator Structure") false false))