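; BP_Controller is the player's camera rig for panning, zooming and clicking on objects in the world with the mouse.
; It adds IMC_Player on BeginPlay; pan and zoom inputs set targets that Tick interpolates into SpringArm location and arm length, with an inverted range mapping for zoom.
; Left click shows a Hand cursor and traces from the camera through the mouse position, offset for the custom cursor, sending ClickMessage to hit ClickInterface actors.
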(event `self.ReceiveBeginPlay`
  (bind _asbp_player_controller (cast `/Game/Controller/BP_PlayerController` (`GameplayStatics.GetPlayerController` 0)))
  (bind _returnvalue (pcsubsystem `EnhancedInputLocalPlayerSubsystem` _asbp_player_controller))
  (`/Engine/EditorBlueprintResources/StandardMacros.IsValid` _returnvalue
    (:`Is Valid`
      (`EnhancedInputSubsystemInterface.AddMappingContext` _returnvalue "/Game/Controller/Input/IMC_Player.IMC_Player" 0 (struct)))
    (:`Is Not Valid`
      (`KismetSystemLibrary.PrintString` "BP_PlayerController: Enhanced Input Local Player Subsystem not valid"))))

(event `EnhancedInput|/Game/Controller/Input/IA_LeftClick`
  (params (ActionValue :type Boolean) (ElapsedSeconds :type "Float (double-precision)") (TriggeredSeconds :type "Float (double-precision)") (InputAction :type "InputAction Object Reference" :default "/Game/Controller/Input/IA_LeftClick.IA_LeftClick"))
  (bind _returnvalue (`GameplayStatics.GetPlayerController` 0))
  (bind (_worldlocation _worlddirection) (`PlayerController.DeprojectMousePositionToWorld` (`GameplayStatics.GetPlayerController` 0)))
  (:`Started`
    (set `PlayerController.CurrentMouseCursor` "Hand" _returnvalue)
    (bind (_outhit _returnvalue_2) (`KismetSystemLibrary.LineTraceSingle` (`SceneComponent.K2_GetComponentLocation` (`self.Camera`)) (+ _worldlocation (* _worlddirection 10000.0) (0.0 -250.0 0.0)) "TraceTypeQuery1"))
    (if _returnvalue_2
      (bind (_bblockinghit _binitialoverlap _time _distance _location _impactpoint _normal _impactnormal _physmat _hitactor) (`GameplayStatics.BreakHitResult` _outhit))
      (if (`KismetSystemLibrary.DoesImplementInterface` _hitactor "/Game/Controller/ClickInterface.ClickInterface_C")
        (message `/Game/Controller/ClickInterface.Click` _hitactor))))
  (:`Completed`
    (set `PlayerController.CurrentMouseCursor` "Default" _returnvalue)))

(event `EnhancedInput|/Game/Controller/Input/IA_RightClick`
  (params (ActionValue :type Boolean) (ElapsedSeconds :type "Float (double-precision)") (TriggeredSeconds :type "Float (double-precision)") (InputAction :type "InputAction Object Reference" :default "/Game/Controller/Input/IA_RightClick.IA_RightClick")))

(event `EnhancedInput|/Game/Controller/Input/IA_CameraPan`
  (params (ActionValue :type "Vector2D Structure") (ElapsedSeconds :type "Float (double-precision)") (TriggeredSeconds :type "Float (double-precision)") (InputAction :type "InputAction Object Reference" :default "/Game/Controller/Input/IA_CameraPan.IA_CameraPan"))
  (bind (_x _y) (`KismetMathLibrary.BreakVector2D` ActionValue))
  (bind _cameraspeed (`self.CameraSpeed`))
  (bind (_desiredcameraoffset_x _desiredcameraoffset_y) (`KismetMathLibrary.BreakVector2D` (`self.DesiredCameraOffset`)))
  (:`Triggered`
    (set `self.DesiredCameraOffset` (`KismetMathLibrary.MakeVector2D` (+ (* _x _cameraspeed) _desiredcameraoffset_x) (+ (* _y _cameraspeed) _desiredcameraoffset_y)))))

(event `EnhancedInput|/Game/Controller/Input/IA_Zoom`
  (params (ActionValue :type "Float (double-precision)") (ElapsedSeconds :type "Float (double-precision)") (TriggeredSeconds :type "Float (double-precision)") (InputAction :type "InputAction Object Reference" :default "/Game/Controller/Input/IA_Zoom.IA_Zoom"))
  (bind (_camerazoomlevels_x _camerazoomlevels_y) (`KismetMathLibrary.BreakVector2D` (`self.CameraZoomLevels`)))
  (:`Triggered`
    (set `self.CameraZoomTarget` (`KismetMathLibrary.FClamp` (+ (`self.CameraZoomCurrent`) (* ActionValue (`self.CameraZoomSpeed`))) _camerazoomlevels_x _camerazoomlevels_y))))

(event `self.ReceiveTick`
  (params (DeltaSeconds :type "Float (single-precision)"))
  (bind _returnvalue (`GameplayStatics.GetWorldDeltaSeconds`))
  (bind _camerasmoothness (`self.CameraSmoothness`))
  (bind (_camerazoomlevels_x _camerazoomlevels_y) (`KismetMathLibrary.BreakVector2D` (`self.CameraZoomLevels`)))
  (bind (_desiredcameraoffset_x _desiredcameraoffset_y) (`KismetMathLibrary.BreakVector2D` (`self.DesiredCameraOffset`)))
  (bind (_relativelocation_x _relativelocation_y) (`KismetMathLibrary.BreakVector` (`SceneComponent.RelativeLocation` (`self.SpringArm`))))
  (`SceneComponent.K2_SetRelativeLocation` (`self.SpringArm`) (`KismetMathLibrary.MakeVector` (`KismetMathLibrary.FInterpTo` _relativelocation_x _desiredcameraoffset_x _returnvalue _camerasmoothness) (`KismetMathLibrary.FInterpTo` _relativelocation_y _desiredcameraoffset_y _returnvalue _camerasmoothness)) false false)
  (bind _output_get (set `self.CameraZoomCurrent` (`KismetMathLibrary.FInterpTo` (`self.CameraZoomCurrent`) (`self.CameraZoomTarget`) (`GameplayStatics.GetWorldDeltaSeconds`) 8.0)))
  (set `SpringArmComponent.TargetArmLength` (`KismetMathLibrary.MapRangeClamped` _output_get _camerazoomlevels_x _camerazoomlevels_y _camerazoomlevels_y _camerazoomlevels_x) (`self.SpringArm`)))

(fn `UserConstructionScript`)