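; Game mode that tracks a CPU budget and triggers a glitch mode when loaded modules exceed it.
; Tick sums CPUCost over loaded BP_Module_Base actors, using DoOnce latches to start and end glitch mode as load crosses CPUMax.
; Glitch mode halves BP_AIPlayer's movement timeline rate, jitters the mouse and repeats an out-of-CPU banner.
; It also drives timed HUD banners and boss UI; a random room-streaming glitch test sits unconnected.
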(event `self.ReceiveBeginPlay`)

(event `self.ReceiveTick`
  (params (DeltaSeconds :type "Float (single-precision)"))
  (`|ExecutionSequence`
    (:`then_0`
      (if (> (`self.BannerDuration`) 0.0)
        (bind _output_get (set `self.BannerDuration` (- (`self.BannerDuration`) DeltaSeconds)))
        (if (<= _output_get 0.0)
          (bind _output_get_2 (set `self.Banner` "NewEnumerator0"))
          (set `/Game/UI/WDG_UI.BannerSelection` _output_get_2 (`self.WDGUI`)))))
    (:`then_1`
      (set `self.CPUCurrent` 0)
      (bind _outactors (`GameplayStatics.GetAllActorsOfClass` "/Game/Modules/Base/BP_Module_Base.BP_Module_Base_C"))
      (for _array_element _outactors
        (if (`/Game/Modules/Base/BP_Module_Base.LevelLoaded` _array_element)
          (set `self.CPUCurrent` (+ (`/Game/Modules/Base/BP_Module_Base.CPUCost` _array_element) (`self.CPUCurrent`)))))
      (if (>= (`self.CPUCurrent`) (`self.CPUMax`))
        (`/Engine/EditorBlueprintResources/StandardMacros.DoOnce` false :!label _label
          (:`Completed`
            (`self.StartGlitchMode`)
            (goto _label_2 :!via `Reset`)))
        (else
          (`/Engine/EditorBlueprintResources/StandardMacros.DoOnce` true :!label _label_2
            (:`Completed`
              (`self.EndGlitchMode`)
              (goto _label :!via `Reset`))))))
    (:`then_2`
      (`self.FuckWithMouse`))))

(event `StartGlitchMode`
  (`|ExecutionSequence`
    (:`then_0`
      (goto _label_4 :!via `Open`))
    (:`then_1`
      (set `self.GlitchMode` true)
      (bind _returnvalue (`GameplayStatics.GetActorOfClass` "/Game/AIPlayer/BP_AIPlayer.BP_AIPlayer_C"))
      (`TimelineComponent.SetPlayRate` (`/Game/AIPlayer/BP_AIPlayer.TL_Move` _returnvalue) 0.5)
      ;[1 1 1] Out of CPU banner
      (bind _asbp_game_mode (cast `/Game/Controller/BP_GameMode` (`GameplayStatics.GetGameMode`) :!label _label_3))
      (`self.SetBannerForDuration` _asbp_game_mode "NewEnumerator5" 3.0)
      (`KismetSystemLibrary.Delay` 2.0)
      (`/Engine/EditorBlueprintResources/StandardMacros.Gate` true :!label _label_4
        (:`Exit`
          (goto _label_3))))))

(event `EndGlitchMode`
  (set `self.GlitchMode` false)
  (bind _returnvalue (`GameplayStatics.GetActorOfClass` "/Game/AIPlayer/BP_AIPlayer.BP_AIPlayer_C"))
  (`TimelineComponent.SetPlayRate` (`/Game/AIPlayer/BP_AIPlayer.TL_Move` _returnvalue) 1.0)
  (goto _label_4 :!via `Close`))

(fn `AddBossToUI`
  (`self.WDGUI`
    (:`then`
      _)
    (:`else`
      (bind _returnvalue (`GameplayStatics.GetActorOfClass` "/Game/UI/BP_Hud.BP_Hud_C"))
      (set `self.WDGUI` (`/Game/UI/BP_Hud.WDGUI` _returnvalue))))
  (`/Game/UI/WDG_UI.AddBossUI` (`self.WDGUI`)))

(fn `AddRemoveCPU`
  (params (Amount :type Integer))
  (set `self.CPUCurrent` (`KismetMathLibrary.Clamp` (+ (`self.CPUCurrent`) Amount) 0 (`self.CPUMax`))))

(fn `FuckWithMouse`
  (bind _returnvalue (`GameplayStatics.GetPlayerController` 0))
  (bind (_locationx _locationy) (`PlayerController.GetMousePosition` _returnvalue))
  (if (`self.GlitchMode`)
    (`PlayerController.SetMouseLocation` _returnvalue (`KismetMathLibrary.FTrunc` (+ _locationx (`KismetMathLibrary.RandomFloatInRange` -20.0 20.0))) (`KismetMathLibrary.FTrunc` (+ _locationy (`KismetMathLibrary.RandomFloatInRange` -20.0 20.0))))))

(fn `IsCPUOverloaded`
  (returns (Overloaded :type Boolean))
  (return (>= (`self.CPUCurrent`) (`self.CPUMax`))))

(fn `SetBannerForDuration`
  (params (Banner :type "/Game/UI/ENUM_BannerSelection Enum" :default "NewEnumerator0") (Duration :type "Float (double-precision)"))
  (`self.WDGUI`
    (:`then`
      _)
    (:`else`
      (bind _returnvalue (`GameplayStatics.GetActorOfClass` "/Game/UI/BP_Hud.BP_Hud_C"))
      (set `self.WDGUI` (`/Game/UI/BP_Hud.WDGUI` _returnvalue))))
  (bind _output_get (set `self.Banner` Banner))
  (set `self.BannerDuration` Duration)
  (set `/Game/UI/WDG_UI.BannerSelection` _output_get (`self.WDGUI`)))

(fn `UserConstructionScript`)